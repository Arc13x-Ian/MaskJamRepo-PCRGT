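; Inventory Blueprint that tracks counts of seeds and items: moss and vine seeds, plus water, wind and bridge items.
; Each has its own Update event that decrements its counter by one, or refuses when it is already zero.
; Results are only printed to screen as debug text; nothing in the graph adds items or notifies other systems.
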(event `UpdateMoss`
  (bind _mossseedcount (`self.MossSeedCount`))
  (if (== _mossseedcount 0)
    (`KismetSystemLibrary.PrintString` "Already Zero Moss")
    (else
      (bind _output_get (set `self.MossSeedCount` (- _mossseedcount 1)))
      (`KismetSystemLibrary.PrintString` (`KismetStringLibrary.Conv_IntToString` _output_get)))))

(event `UpdateVine`
  (bind _vineseedcount (`self.VineSeedCount`))
  (if (== _vineseedcount 0)
    (`KismetSystemLibrary.PrintString` "Already Zero Vine")
    (else
      (bind _output_get (set `self.VineSeedCount` (- _vineseedcount 1)))
      (`KismetSystemLibrary.PrintString` (`KismetStringLibrary.Conv_IntToString` _output_get)))))

(event `UpdateWater`
  (bind _wateritemcount (`self.WaterItemCount`))
  (if (== _wateritemcount 0)
    (`KismetSystemLibrary.PrintString` "Already Zero Water")
    (else
      (bind _output_get (set `self.WaterItemCount` (- _wateritemcount 1)))
      (`KismetSystemLibrary.PrintString` (`KismetStringLibrary.Conv_IntToString` _output_get)))))

(event `UpdateWind`
  (bind _winditemcount (`self.WindItemCount`))
  (if (== _winditemcount 0)
    (`KismetSystemLibrary.PrintString` "Already Zero Wind")
    (else
      (bind _output_get (set `self.WindItemCount` (- _winditemcount 1)))
      (`KismetSystemLibrary.PrintString` (`KismetStringLibrary.Conv_IntToString` _output_get)))))

(event `UpdateBridge`
  (bind _bridgeitemcount (`self.BridgeItemCount`))
  (if (== _bridgeitemcount 0)
    (`KismetSystemLibrary.PrintString` "Already Zero Bridge")
    (else
      (bind _output_get (set `self.BridgeItemCount` (- _bridgeitemcount 1)))
      (`KismetSystemLibrary.PrintString` (`KismetStringLibrary.Conv_IntToString` _output_get)))))