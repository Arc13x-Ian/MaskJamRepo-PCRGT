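; Ruin actor that players cover in moss, counting toward level completion in GM_PlantGame when IsRuin is set.
; GrowMoss spawns a BP_TimerHElper, and MossTick stamps brush material into a render-target mask shown as mesh overlay.
; A timer samples a 16x16 copy for coverage, normalised by used UV space, completing the ruin at CompletionThreshold and showing the win screen after the last.
; Another timer line-traces mossy spots to grow plant meshes.
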(event `self.ReceiveBeginPlay`
  (bind _mossmaskresolution (`self.MossMaskResolution`))
  (`KismetSystemLibrary.Delay` 1.0)
  (if (`self.Is Ruin?`)
    (`|ExecutionSequence`
      (:`then_0`
        ; Create and apply moss mask material to main mesh
        (bind _returnvalue (`KismetRenderingLibrary.CreateRenderTarget2D` _mossmaskresolution _mossmaskresolution "RTF_R8" (struct :`A` 1.0) true))
        (bind _output_get (set `self.RenderTargetCanvas` _returnvalue))
        (`KismetRenderingLibrary.ClearRenderTarget2D` _output_get (struct))
        (bind _returnvalue_2 (`KismetMaterialLibrary.CreateDynamicMaterialInstance` "/Game/LukesStuff/M_MossMap.M_MossMap"))
        (bind _output_get_2 (set `self.MossMask` _returnvalue_2))
        (`MaterialInstanceDynamic.SetTextureParameterValue` _output_get_2 "Render Target" (`self.RenderTargetCanvas`))
        (`MeshComponent.SetOverlayMaterial` (`self.StaticMesh`) (`self.MossMask`))
        (bind _asgm_plant_game (cast `/Game/LukesStuff/GM_PlantGame` (`GameplayStatics.GetGameMode`)))
        (set `self.As GM Plant Game` _asgm_plant_game))
      (:`then_1`
        ; Calculate how much of the texture is "texture" and how much is blank space (Uses alpha for this)
        (bind _returnvalue_3 (`CanvasRenderTarget2D.CreateCanvasRenderTarget2D` "/Script/Engine.CanvasRenderTarget2D" 16 16))
        (bind (_canvas _size _context) (`KismetRenderingLibrary.BeginDrawCanvasToRenderTarget` _returnvalue_3))
        (`Canvas.K2_DrawMaterial` _canvas (`PrimitiveComponent.GetMaterial` (`self.StaticMesh`) 0) (0.0 0.0) (16.0 16.0) (0.0 0.0) (1.0 1.0) 0.0 (0.5 0.5))
        (`KismetRenderingLibrary.EndDrawCanvasToRenderTarget` _context)
        (bind _outsamples (`KismetRenderingLibrary.ReadRenderTarget` _returnvalue_3))
        (set `self.PercentCounter` 0)
        (for _array_element _outsamples
          (if (< (/ (`KismetMathLibrary.Conv_ByteToDouble` (`.A` (break `Color` _array_element))) 255.0) 0.9)
            (`/Engine/EditorBlueprintResources/StandardMacros.IncrementInt` (`self.PercentCounter`))))
        (set `self.TexturePercent` (/ (`KismetMathLibrary.Conv_IntToDouble` (`self.PercentCounter`)) 255.0)))
      (:`then_2`
        ; Create lower resolution "calculation" render target
        (bind _returnvalue_4 (`CanvasRenderTarget2D.CreateCanvasRenderTarget2D` "/Script/Engine.CanvasRenderTarget2D" 16 16))
        (set `self.PercentSampler` _returnvalue_4)
        (bind _returnvalue_5 (`KismetMaterialLibrary.CreateDynamicMaterialInstance` "/Game/LukesStuff/M_MossMap.M_MossMap"))
        (`MaterialInstanceDynamic.SetTextureParameterValue` _returnvalue_5 "Render Target" (`self.PercentSampler`))
        (`PrimitiveComponent.SetMaterial` (`self.Plane`) 0 _returnvalue_5))
      (:`then_4`
        ; Misc stuff
        (bind _returnvalue_6 (`KismetSystemLibrary.K2_SetTimerDelegate` (delegate `Calculate AmountCovered`) 0.2 true))
        (`PrimitiveComponent.SetMaterial` (`self.Plane1`) 0 (`self.MossMask`))
        (set `self.LoopingTimerHandle` _returnvalue_6)
        (`KismetSystemLibrary.K2_SetTimerDelegate` (delegate `GrowPlantCheck`) 0.1 true))
      (:`then_5`
        ; force blueprint to be changed
        (bind _as_gm_plant_game (`self.As GM Plant Game`)
          (:`then`
            (`/Engine/EditorBlueprintResources/StandardMacros.IncrementInt` (`/Game/LukesStuff/GM_PlantGame.TotalRuins` _as_gm_plant_game)))
          (:`else`))))))

(event `/Game/LukesStuff/BPI_GrowMoss.Grow Moss`
  (params (`UV Location` :type "Vector2D Structure") (Size :type "Float (double-precision)"))
  (bind (_returnvalue_x _returnvalue_y _returnvalue_z) (`KismetMathLibrary.BreakVector` (`self.GetActorScale3D`)))
  ; Moss growth event
  (set `self.ShouldSpawnPlants` true)
  (bind _returnvalue (`|SpawnActorFromClass` "/Game/LukesStuff/BP_TimerHElper.BP_TimerHElper_C" (`KismetMathLibrary.MakeTransform` (0.0 0.0 0.0)) "Undefined" "MultiplyWithRoot" null null))
  (set `/Game/LukesStuff/BP_TimerHElper.Parent` self _returnvalue)
  (set `/Game/LukesStuff/BP_TimerHElper.Size` (/ Size (/ (+ _returnvalue_x _returnvalue_y _returnvalue_z) 3.0)) _returnvalue)
  (set `/Game/LukesStuff/BP_TimerHElper.UV Location` `UV Location` _returnvalue)
  (bind _returnvalue_2 (`KismetMaterialLibrary.CreateDynamicMaterialInstance` "/Game/LukesStuff/M_Brush.M_Brush"))
  (set `self.StampTexture` _returnvalue_2)
  (`MaterialInstanceDynamic.SetVectorParameterValue` _returnvalue_2 "Noise" (make `LinearColor` 0.0 0.0 0.0 1.0))
  (message `AudioParameterControllerInterface.SetFloatParameter` _returnvalue_2 "WarpStrength" 0.0)
  (`/Game/LukesStuff/BP_TimerHElper.Init` _returnvalue))

(event `MossTick`
  (params (Size :type "Float (double-precision)") (`UV Location` :type "Vector2D Structure"))
  (bind _returnvalue (/ Size 2.0))
  (bind _mossmaskresolution (`self.MossMaskResolution`))
  ; Moss growth event
  (bind (_canvas _size _context) (`KismetRenderingLibrary.BeginDrawCanvasToRenderTarget` (`self.RenderTargetCanvas`)))
  (`Canvas.K2_DrawMaterial` _canvas (`self.StampTexture`) (- (* `UV Location` (`KismetMathLibrary.MakeVector2D` (`KismetMathLibrary.Conv_IntToDouble` _mossmaskresolution) (`KismetMathLibrary.Conv_IntToDouble` _mossmaskresolution))) (`KismetMathLibrary.MakeVector2D` _returnvalue _returnvalue)) (`KismetMathLibrary.MakeVector2D` Size Size) (0.0 0.0) (1.0 1.0) 0.0 (0.5 0.5))
  (`KismetSystemLibrary.PrintString` "Hello" false false (struct :`G` 0.66 :`B` 1.0 :`A` 1.0) Size)
  (`KismetRenderingLibrary.EndDrawCanvasToRenderTarget` _context))

(event `Calculate AmountCovered`
  (`|ExecutionSequence`
    (:`then_0`
      ; Function that calculates the % of mesh covered
      (`|ExecutionSequence`
        (:`then_0`
          (`KismetRenderingLibrary.ClearRenderTarget2D` (`self.PercentSampler`))
          (bind (_canvas _size _context) (`KismetRenderingLibrary.BeginDrawCanvasToRenderTarget` (`self.PercentSampler`)))
          (`Canvas.K2_DrawMaterial` _canvas (`self.MossMask`) (0.0 0.0) (16.0 16.0) (0.0 0.0) (1.0 1.0) 0.0 (0.5 0.5))
          (`KismetRenderingLibrary.EndDrawCanvasToRenderTarget` _context)
          (bind _outsamples (`KismetRenderingLibrary.ReadRenderTarget` (`self.PercentSampler`)))
          (set `self.PercentCounter` 0)
          (for _array_element _outsamples
            (if (< (/ (`KismetMathLibrary.Conv_ByteToDouble` (`.A` (break `Color` _array_element))) 255.0) 0.9)
              (`/Engine/EditorBlueprintResources/StandardMacros.IncrementInt` (`self.PercentCounter`))))
          (bind _output_get (set `self.PercentOfMeshCovered` (* (/ (/ (`KismetMathLibrary.Conv_IntToDouble` (`self.PercentCounter`)) 255.0) (`self.TexturePercent`)) 100.0)))
          (`KismetSystemLibrary.PrintString` (`KismetStringLibrary.Conv_DoubleToString` _output_get)))
        (:`then_1`
          (if (>= (`self.PercentOfMeshCovered`) (`self.CompletionThreshold`))
            (`KismetRenderingLibrary.ClearRenderTarget2D` (`self.RenderTargetCanvas`) (struct :`R` 1.0 :`G` 1.0 :`B` 1.0 :`A` 1.0))
            ;[1 0.9256 0] WIN CONDITION
            (`ActorComponent.Activate` (`self.N_RuinCompleted`) false)
            (`KismetSystemLibrary.K2_ClearAndInvalidateTimerHandle` (`self.LoopingTimerHandle`))
            (bind _as_gm_plant_game (`self.As GM Plant Game`)
              (:`then`
                (`/Engine/EditorBlueprintResources/StandardMacros.IncrementInt` (`/Game/LukesStuff/GM_PlantGame.CompletedRuins` _as_gm_plant_game)
                  (:`  `
                    (if (>= (`/Game/LukesStuff/GM_PlantGame.CompletedRuins` _as_gm_plant_game) (`/Game/LukesStuff/GM_PlantGame.TotalRuins` _as_gm_plant_game))
                      (`KismetSystemLibrary.PrintString` "LEVEL COMPLETED" true true (struct :`R` 1.0 :`G` 0.925603 :`A` 1.0) 10.0)
                      (`NiagaraFunctionLibrary.SpawnSystemAtLocation` "/Game/LukesStuff/N_LevelCompleted.N_LevelCompleted" (`self.K2_GetActorLocation` (`GameplayStatics.GetPlayerCharacter` 0)) (struct) (1.25 1.25 1.25))
                      (`KismetSystemLibrary.Delay` 1.0)
                      (bind _returnvalue (`|CreateWidget` "/Game/UI/WBP_WinScreen.WBP_WinScreen_C"))
                      (`UserWidget.AddToViewport` _returnvalue 0)))))
              (:`else`))))))))

(event `GrowPlantCheck`
  (bind _returnvalue (`self.GetTransform`))
  (bind _plantlocations (`self.PlantLocations`))
  (bind _plantcountpermesh (`self.PlantCountPerMesh`))
  (if (`self.ShouldSpawnPlants`)
    (for _ (range 11)
      (bind _outhit (`KismetSystemLibrary.LineTraceSingleForObjects` :`Start` (+ (`self.K2_GetActorLocation`) (* (`KismetMathLibrary.RandomUnitVector`) 2500.0)) :`End` (`self.K2_GetActorLocation`) :`ObjectTypes` (`|MakeArray` "ObjectTypeQuery2" :!type "EObjectTypeQuery Enum") :`bIgnoreSelf` false))
      (bind (_bblockinghit _binitialoverlap _time _distance _location _impactpoint _normal _impactnormal _physmat _hitactor) (`GameplayStatics.BreakHitResult` _outhit))
      (if (== _hitactor self)
        (bind _uv (`GameplayStatics.FindCollisionUV` _outhit))
        (bind (_returnvalue_x _returnvalue_y) (`KismetMathLibrary.BreakVector2D` (* _uv (16.0 16.0))))
        (bind _returnvalue_2 (`KismetRenderingLibrary.ReadRenderTargetPixel` (`self.PercentSampler`) (`KismetMathLibrary.FTrunc` _returnvalue_x) (`KismetMathLibrary.FTrunc` _returnvalue_y)))
        (if (< (`KismetMathLibrary.Conv_ByteToDouble` (`.A` (break `Color` _returnvalue_2))) 0.9)
          (bind _returnvalue_3 (/ (`KismetMathLibrary.ToRounded2D` (* _uv _plantcountpermesh)) _plantcountpermesh))
          (if (not (`KismetArrayLibrary.Array_Contains` _plantlocations _returnvalue_3))
            (`KismetArrayLibrary.Array_Add` _plantlocations _returnvalue_3)
            (bind _returnvalue_4 (`AddComponent|NODE_AddStaticMeshComponent-0` :`RelativeTransform` (`KismetMathLibrary.MakeTransform` (`KismetMathLibrary.InverseTransformLocation` _returnvalue _location) (`KismetMathLibrary.InverseTransformRotation` _returnvalue (`KismetMathLibrary.MakeRotFromZX` (`KismetMathLibrary.Normal` _impactnormal) (`self.GetActorUpVector`))) (`KismetMathLibrary.Conv_DoubleToVector` 0.05))))
            (`StaticMeshComponent.SetStaticMesh` _returnvalue_4 (`KismetArrayLibrary.Array_Random` (`self.PlantMeshes`)))
            (bind (_direction _newtrack_0) (`Timeline|Growth` :!via `PlayFromStart`)
              (:`Update`
                (`SceneComponent.SetRelativeScale3D` _returnvalue_4 (`KismetMathLibrary.Conv_DoubleToVector` (`KismetMathLibrary.Lerp` 0.0 0.2 _newtrack_0)))))))))))

(fn `UserConstructionScript`
  (`StaticMeshComponent.SetStaticMesh` (`self.StaticMesh`) (`self.Mesh`)))