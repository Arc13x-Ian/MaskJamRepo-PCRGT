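; BP_TimerHElper is a short-lived helper actor that drives a timed moss effect on its Parent at a UV location.
; Init runs a delayed loop that repeatedly calls MossTick with the UV location and CalculateSize's result, then destroys the actor once the counter hits its limit.
; CalculateSize contains a curve-based scaling of Size by the counter, but that expression is marked unused.
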(event `Init`
  (if (< (`self.Counter`) 20) :!label _label
    (`/Game/LukesStuff/BP_Ruin.MossTick` (`self.Parent`) (* (`self.Size`) (`KismetMathLibrary.Lerp` 0.0 1.0 (`CurveFloat.GetFloatValue` (`self.Curve`) (* (`self.Counter`) 0.1)))) (`self.UV Location`))
    (`KismetSystemLibrary.Delay` 0.05)
    (`/Engine/EditorBlueprintResources/StandardMacros.IncrementInt` (`self.Counter`)
      (:`  `
        (goto _label)))
    (else
      (`self.K2_DestroyActor`))))

(fn `UserConstructionScript`)