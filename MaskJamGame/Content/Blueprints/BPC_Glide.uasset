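; Glide component for BP_ThirdPersonCharacter that adds low-gravity gliding and transitions to and from climbing.
; StartGlide retunes CharacterMovement and gives an upward boost, while StopGlide restores defaults cached at BeginPlay and a fixed walk speed.
; While gliding, Tick pushes the character forward, traces down for floor, and sphere-traces for "Can Climb" actors to attach to in Flying mode.
; Gliding from a climb launches backward and re-enables climbing after a short timer.
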(event `self.ReceiveBeginPlay`
  (bind _character_movement (`self.Character Movement`))
  ; Glide
  (bind _asbp_third_person_character (cast `/Game/ThirdPerson/Blueprints/BP_ThirdPersonCharacter` (`self.GetOwner`)))
  (set `self.As BP Third Person Character` _asbp_third_person_character)
  (bind _output_get (set `self.Character Movement` (`Character.CharacterMovement` _asbp_third_person_character)))
  (set `self.Default Braking Deceleration Falling` (`CharacterMovementComponent.BrakingDecelerationFalling` _output_get))
  (set `self.Default Air Control` (`CharacterMovementComponent.AirControl` _character_movement))
  (set `self.Default Gravity Scale` (`CharacterMovementComponent.GravityScale` _character_movement))
  (set `self.Original Orient Rotation To Movement` (`CharacterMovementComponent.bOrientRotationToMovement` (`self.Character Movement`)))
  (set `self.Original Use Controller Rotation Yaw` (`Pawn.bUseControllerRotationYaw` (`self.As BP Third Person Character`))))

(event `Check For Floor`
  (bind _as_bp_third_person_character (`self.As BP Third Person Character`))
  (bind _returnvalue (`Actor.K2_GetActorLocation` _as_bp_third_person_character))
  ; Glide
  (bind (_outhit _returnvalue_2) (`KismetSystemLibrary.LineTraceSingleForObjects` _returnvalue (+ _returnvalue (* (* (`Actor.GetActorUpVector` _as_bp_third_person_character) -1.0) 100.0)) (`|MakeArray` "ObjectTypeQuery1" "ObjectTypeQuery2" :!type "EObjectTypeQuery Enum") :!label _label))
  (if _returnvalue_2
    (set `/Game/ThirdPerson/Blueprints/BP_ThirdPersonCharacter.Action` "NewEnumerator0" (`self.As BP Third Person Character`))
    (`self.Stop Glide`)))

(event `self.ReceiveTick`
  (params (DeltaSeconds :type "Float (single-precision)"))
  (bind _as_bp_third_person_character (`self.As BP Third Person Character`))
  (bind _as_bp_third_person_character_2 (`self.As BP Third Person Character`))
  (bind _character_movement (`self.Character Movement`))
  (bind _returnvalue (`Actor.K2_GetActorLocation` (`self.As BP Third Person Character`)))
  (bind (_returnvalue_x _returnvalue_y) (`KismetMathLibrary.BreakVector` (`KismetMathLibrary.GetForwardVector` (`Actor.K2_GetActorRotation` _as_bp_third_person_character))))
  ; Glide
  (bind _as_bp_third_person_character_3 (`self.As BP Third Person Character`)
    (:`then`
      (switch `/Game/ThirdPerson/Blueprints/E_Action` (`/Game/ThirdPerson/Blueprints/BP_ThirdPersonCharacter.Action` _as_bp_third_person_character_3)
        (:`NewEnumerator0`
          (`self.Check For Floor`))
        (:`NewEnumerator1`
          (set `self.Can Climb?` false))
        (:`NewEnumerator2`
          (`Pawn.AddMovementInput` _as_bp_third_person_character (`KismetMathLibrary.MakeVector` _returnvalue_x _returnvalue_y) 1.0 false)
          (`|ExecutionSequence`
            (:`then_0`
              (if (`self.Can Climb?`)
                (bind (_outhit _returnvalue_2) (`KismetSystemLibrary.SphereTraceSingleForObjects` _returnvalue _returnvalue 75.0 (`|MakeArray` "ObjectTypeQuery1" "ObjectTypeQuery2" "ObjectTypeQuery4" :!type "EObjectTypeQuery Enum")))
                (if _returnvalue_2
                  (bind (_bblockinghit _binitialoverlap _time _distance _location _impactpoint _normal _impactnormal _physmat _hitactor) (`GameplayStatics.BreakHitResult` _outhit))
                  (if (`Actor.ActorHasTag` _hitactor "Can Climb")
                    (`self.Stop Glide`)
                    (`CharacterMovementComponent.SetMovementMode` (`self.Character Movement`) "MOVE_Flying" 0)
                    (set `/Game/ThirdPerson/Blueprints/BP_ThirdPersonCharacter.Action` "NewEnumerator1" _as_bp_third_person_character_2)
                    (set `Pawn.bUseControllerRotationYaw` false _as_bp_third_person_character_2)
                    (set `CharacterMovementComponent.bOrientRotationToMovement` false _character_movement)
                    (set `CharacterMovementComponent.BrakingDecelerationFlying` 99999.0 _character_movement)
                    (set `CharacterMovementComponent.MaxFlySpeed` 150.0 _character_movement)
                    (`KismetSystemLibrary.MoveComponentTo` (`Character.CapsuleComponent` (`self.As BP Third Person Character`)) (+ (+ _impactpoint (* _impactnormal (`CapsuleComponent.CapsuleRadius` (`Character.CapsuleComponent` (`self.As BP Third Person Character`))))) (0.0 0.0 50.0)) (`KismetMathLibrary.MakeRotFromX` (* _impactnormal -1.0)) false false 0.4)))))
            (:`then_1`
              (goto _label))))))
    (:`else`)))

(event `Start Glide`
  (bind _character_movement (`self.Character Movement`))
  (bind (_velocity_x _velocity_y) (`KismetMathLibrary.BreakVector` (`MovementComponent.Velocity` _character_movement)))
  ; Glide
  (set `CharacterMovementComponent.BrakingDecelerationFalling` 0.0 _character_movement)
  (set `CharacterMovementComponent.AirControl` 0.7 _character_movement)
  (set `CharacterMovementComponent.GravityScale` 0.1 _character_movement)
  (set `CharacterMovementComponent.bOrientRotationToMovement` false _character_movement)
  (set `MovementComponent.Velocity` (`KismetMathLibrary.MakeVector` _velocity_x _velocity_y 400.0) _character_movement)
  (set `Pawn.bUseControllerRotationYaw` true (`self.As BP Third Person Character`))
  (`self.Glide From Climb`)
  (set `/Game/ThirdPerson/Blueprints/BP_ThirdPersonCharacter.Action` "NewEnumerator2" (`self.As BP Third Person Character`))
  (set `CharacterMovementComponent.MaxWalkSpeed` 1500.0 (`self.Character Movement`)))

(event `Stop Glide`
  (bind _character_movement (`self.Character Movement`))
  ; Glide
  (set `CharacterMovementComponent.BrakingDecelerationFalling` (`self.Default Braking Deceleration Falling`) _character_movement)
  (set `CharacterMovementComponent.AirControl` (`self.Default Air Control`) _character_movement)
  (set `CharacterMovementComponent.GravityScale` (`self.Default Gravity Scale`) _character_movement)
  (set `CharacterMovementComponent.bOrientRotationToMovement` (`self.Original Orient Rotation To Movement`) _character_movement)
  (set `Pawn.bUseControllerRotationYaw` (`self.Original Use Controller Rotation Yaw`) (`self.As BP Third Person Character`))
  (set `CharacterMovementComponent.MaxWalkSpeed` 600.0 (`self.Character Movement`)))

(event `Glide From Climb`
  (bind _as_bp_third_person_character (`self.As BP Third Person Character`))
  (switch `/Game/ThirdPerson/Blueprints/E_Action` (`/Game/ThirdPerson/Blueprints/BP_ThirdPersonCharacter.Action` (`self.As BP Third Person Character`))
    (:`NewEnumerator1`
      (`/Engine/EditorBlueprintResources/StandardMacros.DoOnce` false :!label _label_2
        (:`Completed`
          (set `self.Can Climb?` false)
          (`Character.LaunchCharacter` _as_bp_third_person_character (* (* (`Actor.GetActorForwardVector` _as_bp_third_person_character) -1.0) 1000.0) true true)
          (`KismetSystemLibrary.K2_SetTimerDelegate` (delegate `Can Climb Timer`) 1.0))))))

(event `Reset Climb Jump`
  (goto _label_2 :!via `Reset`))

(event `Can Climb Timer`
  (set `self.Can Climb?` true)
  (`self.Reset Climb Jump`))