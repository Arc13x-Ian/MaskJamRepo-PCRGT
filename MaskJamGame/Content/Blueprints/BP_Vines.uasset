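; BP_Vines is an actor that builds a vertical column of static mesh segments, presumably vines, when play begins.
; BeginPlay seeds an array with the Cube component, then loops up to MaxVines, spawning each new component a fixed height above the previous entry.
; Each segment is uniformly scaled, set to the WorldStatic collision type and appended to the array to anchor the next one.
; The construction script is empty.
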(event `self.ReceiveBeginPlay`
  (`KismetArrayLibrary.Array_Add` (`self.Static Mesh Array`) (`self.Cube`))
  (for _index (range (+ (`self.Max Vines`) 1))
    (bind _returnvalue (`AddComponent|NODE_AddStaticMeshComponent-0` :`RelativeTransform` (`KismetMathLibrary.MakeTransform` (+ (`SceneComponent.RelativeLocation` (`|GetArrayItem` (`self.Static Mesh Array`) _index)) (0.0 0.0 225.0)) (struct) (4.0 4.0 4.0))))
    (`PrimitiveComponent.SetCollisionObjectType` _returnvalue "ECC_WorldStatic")
    (`KismetArrayLibrary.Array_Add` (`self.Static Mesh Array`) _returnvalue)))

(fn `UserConstructionScript`)