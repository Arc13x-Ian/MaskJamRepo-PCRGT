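; BP_MasterTile is a tile Blueprint in the puzzle generator that can be turned into a ruin.
; ToggleIsRuin stores the flag and, when true, spawns a BP_Ruin at the tile's transform with a random mesh from RuinMeshPool, keeping it in RuinRef.
; A false value only updates the flag and leaves any spawned ruin in place.
; Disconnected nodes that set collision and mesh on the tile's own RuinMesh component never run.
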(event `ToggleIsRuin`
  (params (IsRuin :type Boolean))
  (bind _output_get (set `self.IsRuin` IsRuin))
  (if _output_get
    (bind _returnvalue (`|SpawnActorFromClass` "/Game/CoverMechanicThingy/BP_Ruin.BP_Ruin_C" (`self.GetTransform`) "Undefined" "MultiplyWithRoot" null (`KismetArrayLibrary.Array_Random` (`self.RuinMeshPool`)) null))
    (set `self.RuinRef` _returnvalue)))

(fn `UserConstructionScript`)