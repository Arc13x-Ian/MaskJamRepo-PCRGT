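; Puzzle map generator actor that builds a random tile layout with a player spawn, ruins and a water source on BeginPlay.
; It spawns randomly rotated BP_MasterTiles up to MaxPieces, tracking grid coordinates to reject occupied locations.
; Shuffled tile lists then pick ruins, using the GameInstance's count and skipping the spawn tile, and a non-ruin tile for BP_WaterSource.
; An older weighted-class generation path remains, unexecuted.
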(event `self.ReceiveBeginPlay`
  (bind _asgi_plant_game_instance (cast `/Game/LukesStuff/GI_PlantGameInstance` (`GameplayStatics.GetGameInstance`))
    (:`then`
      (set `self.GameInstance_Ref` _asgi_plant_game_instance)
      (`self.TileGeneration`))
    (:`CastFailed`
      (`KismetSystemLibrary.PrintString` "PuzzleRandomGenerator:   Invalid GameInstance cast!"))))

(event `TileGeneration`
  ; Clear all ref arrays
  (`KismetArrayLibrary.Array_Clear` (`self.AllTiles`))
  (`KismetArrayLibrary.Array_Clear` (`self.AllRuinTiles`))
  (`KismetArrayLibrary.Array_Clear` (`self.Grid Data`))
  ; Spawn initial tile and store a reference to it
  (bind _tilecreatedref (`self.SpawnNewTile` (`KismetMathLibrary.MakeTransform` (`SceneComponent.K2_GetComponentLocation` (`self.DefaultSceneRoot`)) (select `int` (`KismetMathLibrary.RandomInteger` 3) :`0` (struct) :`1` (struct :`Yaw` 90.0) :`2` (struct :`Yaw` 180.0) :`3` (struct :`Yaw` 270.0) :!type "Rotator Structure") (`KismetMathLibrary.Conv_DoubleToVector` (`self.ScaleTemp`)))))
  (bind _output_get (set `self.PlayerSpawnTile` _tilecreatedref))
  (set `/Game/Blueprints/Puzzle_Generator/BP_MasterTile.IsPlayerSpawnTile` true _output_get)
  ; If total tiles is still below max number of tiles
  (while (< (`self.CurrentTileCount`) (`self.Max Pieces`))
    ; Get random new spawn location
    (bind _output_get_2 (set `self.Spawn Location` (`self.GetRandomNextSpawnLocation`)))
    ; Is this spawn location already occupied?
    (if (`KismetArrayLibrary.Array_Contains` (`self.Grid Data`) (/ (`KismetMathLibrary.MakeVector2D` (.x _output_get_2) (.y _output_get_2)) (`self.Tile Size`)))
      (set `self.Spawn Location` (0.0 0.0 0.0)) ; Reset spawn location
      (else
        ; Spawn new tile
        (`self.SpawnNewTile` (`KismetMathLibrary.MakeTransform` (`self.Spawn Location`) (select `int` (`KismetMathLibrary.RandomInteger` 3) :`0` (struct) :`1` (struct :`Yaw` 90.0) :`2` (struct :`Yaw` 180.0) :`3` (struct :`Yaw` 270.0) :!type "Rotator Structure") (`KismetMathLibrary.Conv_DoubleToVector` (`self.ScaleTemp`))))
        (`/Engine/EditorBlueprintResources/StandardMacros.IncrementInt` (`self.CurrentTileCount`)))))
  ; After all tiles are placed, determine which ones will be ruins
  (`self.DetermineRuinTiles`))

(event `DetermineRuinTiles`
  ; Generate ruins
  (`KismetArrayLibrary.Array_Shuffle` (`self.AllTiles`)) ; Randomize the order of the list of tiles
  (for (_array_element _array_index) (`self.AllTiles`)
    (if (< _array_index (`/Game/LukesStuff/GI_PlantGameInstance.RuinsToSpawn` (`self.GameInstance_Ref`)))
      (if (!= _array_element (`self.PlayerSpawnTile`))
        (`/Game/Blueprints/Puzzle_Generator/BP_MasterTile.ToggleIsRuin` _array_element true) ; Tell that tile to become a ruin
        (`KismetArrayLibrary.Array_Add` (`self.AllRuinTiles`) _array_element) ; Store reference to ruin tile
      )
      (else
        (`/Game/Blueprints/Puzzle_Generator/BP_MasterTile.ToggleIsRuin` _array_element false))))
  (`self.SpawnWaterPool`) ; Call to spawn water pool
)

(event `StopRuinSpawning`
  ; Generate ruins
)

(event `SpawnWaterPool`
  (bind _alltiles (`self.AllTiles`))
  ; Spawn the water pool
  (`KismetArrayLibrary.Array_Shuffle` _alltiles)
  (for _array_element _alltiles :!label _label
    (if (not (`KismetArrayLibrary.Array_Contains` (`self.AllRuinTiles`) _array_element))
      (bind _output_get (set `self.WaterPoolTile_Ref` _array_element))
      (`|SpawnActorFromClass` "/Game/Blueprints/BP_WaterSource.BP_WaterSource_C" (`self.GetTransform` _output_get) "AlwaysSpawn" "MultiplyWithRoot" null null)
      (`self.FinishWaterPoolSpawn`)))
  (`self.PrintMapDetails`) ; Print map generation details
)

(event `FinishWaterPoolSpawn`
  ; Spawn the water pool
  (goto _label :!via `Break`))

(event `PrintMapDetails`)

(event `Set Ruin Probability`
  ;[1 0 0 0.5] Previous
  (for _ (range 1 901)
    (`KismetArrayLibrary.Array_Add` (`self.Land Actor Selector`) "/Game/Blueprints/Puzzle_Generator/BP_Wasteland.BP_Wasteland_C"))
  (for _ (range 1 11)
    (`KismetArrayLibrary.Array_Add` (`self.Land Actor Selector`))))

(fn `Check For Ruins`
  (params (`Ruin?` :type "Object Object Reference"))
  (if (== (`GameplayStatics.GetObjectClass` `Ruin?`) null)
    (`|ExecutionSequence`
      (:`then_0`
        (bind _result (`/Engine/EditorBlueprintResources/StandardMacros.IncrementInt` (`self.Ruin Count`))
          (:`  `
            (if (== _result (`self.Max Ruins`))
              (`KismetArrayLibrary.Array_RemoveItem` (`self.Land Actor Selector`)))))))))

(fn `PrintDebugMapDetails`
  (`KismetSystemLibrary.PrintString` (`KismetStringLibrary.Concat_StrStr` "Tile Size:  " (`KismetStringLibrary.Conv_DoubleToString` (* (`self.Tile Size`) (`self.ScaleTemp`)))) true true (struct :`R` 0.422554 :`B` 1.0 :`A` 1.0) 5.0)
  (`KismetSystemLibrary.PrintString` (`KismetStringLibrary.Concat_StrStr` "Total Tile Count:   :  " (`KismetStringLibrary.Conv_IntToString` (`KismetArrayLibrary.Array_Length` (`self.AllTiles`)))) true true (struct :`R` 0.422554 :`B` 1.0 :`A` 1.0) 5.0)
  (`KismetSystemLibrary.PrintString` (`KismetStringLibrary.Concat_StrStr` "Total Ruin Count:   :  " (`KismetStringLibrary.Conv_IntToString` (`KismetArrayLibrary.Array_Length` (`self.AllRuinTiles`)))) true true (struct :`R` 0.422554 :`B` 1.0 :`A` 1.0) 5.0))

(fn `SpawnNewTile`
  (params (SpawnTransform :type "Transform Structure"))
  (returns (TileCreatedRef :type "/Game/Blueprints/Puzzle_Generator/BP_MasterTile Object Reference"))
  (bind _returnvalue (`|SpawnActorFromClass` "/Game/Blueprints/Puzzle_Generator/BP_MasterTile.BP_MasterTile_C" SpawnTransform "Undefined" "MultiplyWithRoot" null null))
  (`KismetArrayLibrary.Array_Add` (`self.AllTiles`) _returnvalue)
  (`KismetArrayLibrary.Array_AddUnique` (`self.Grid Data`) (/ (`KismetMathLibrary.MakeVector2D` (.x (`SceneComponent.K2_GetComponentLocation` (`Actor.RootComponent` _returnvalue))) (.y (`SceneComponent.K2_GetComponentLocation` (`Actor.RootComponent` _returnvalue)))) (`self.Tile Size`))) ; Store its world position
  (return _returnvalue))

(fn `UserConstructionScript`)