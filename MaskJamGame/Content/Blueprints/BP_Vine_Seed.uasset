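; BP_Vine_Seed is a seed actor that turns into vines where it hits something.
; On Hit, unless the other actor matches BP_Ruin, it spawns a double-scale, unrotated BP_Vines at the hit location and destroys itself.
; Tick also runs a debug-drawn sphere trace around the seed, but its result drives nothing.
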(event `self.ReceiveTick`
  (params (DeltaSeconds :type "Float (single-precision)"))
  (bind _returnvalue (`self.K2_GetActorLocation`))
  (bind (_outhit _returnvalue_2) (`KismetSystemLibrary.SphereTraceSingleForObjects` :`Start` _returnvalue :`End` _returnvalue :`Radius` 50.0 :`ObjectTypes` (`|MakeArray` "ObjectTypeQuery1" "ObjectTypeQuery2" "ObjectTypeQuery4" :!type "EObjectTypeQuery Enum") :`DrawDebugType` "ForOneFrame"))
  (if _returnvalue_2
    _))

(event `self.ReceiveHit`
  (params (MyComp :type "PrimitiveComponent Object Reference") (Other :type "Actor Object Reference") (OtherComp :type "PrimitiveComponent Object Reference") (bSelfMoved :type Boolean) (HitLocation :type "Vector Structure") (HitNormal :type "Vector Structure") (NormalImpulse :type "Vector Structure") (Hit :type "HitResult Structure (by ref)"))
  (if (not (== Other "/Game/LukesStuff/BP_Ruin.BP_Ruin"))
    (`|SpawnActorFromClass` "/Game/Blueprints/BP_Vines.BP_Vines_C" (`KismetMathLibrary.MakeTransform` HitLocation (struct) (2.0 2.0 2.0)) "Undefined" "MultiplyWithRoot" null null)
    (`self.K2_DestroyActor`)))

(fn `UserConstructionScript`)