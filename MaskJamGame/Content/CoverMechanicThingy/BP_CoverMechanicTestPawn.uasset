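; Test pawn for the cover mechanic that paints moss onto objects it aims at on left mouse click.
; Each click runs a complex, debug-drawn line trace against WorldDynamic objects, intended to span PaintDistance along the actor's forward vector.
; It uses Find Collision UV to read the hit's texture coordinates.
; Hit actors implementing BPI_GrowMoss receive that UV and a fixed brush size through GrowMoss.
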(event `Key|LeftMouseButton`
  (params (Key :type "Key Structure"))
  (:`Pressed`
    (bind _outhit (`KismetSystemLibrary.LineTraceSingleForObjects` :`Start` (`self.K2_GetActorLocation`) :`End` (+ (`self.K2_GetActorLocation`) (* (`self.GetActorForwardVector`) (`self.PaintDistance`))) :`ObjectTypes` (`|MakeArray` "ObjectTypeQuery2" :!type "EObjectTypeQuery Enum") :`bTraceComplex` true :`DrawDebugType` "Persistent"))
    (bind _uv (`GameplayStatics.FindCollisionUV` _outhit))
    (bind _returnvalue (`KismetMathLibrary.MakeVector2D` (`KismetMathLibrary.BreakVector2D` _uv) (`.Y` (`KismetMathLibrary.BreakVector2D` _uv))))
    (`KismetSystemLibrary.PrintString` (`KismetStringLibrary.Conv_Vector2dToString` _returnvalue) false)
    (bind (_bblockinghit _binitialoverlap _time _distance _location _impactpoint _normal _impactnormal _physmat _hitactor) (`GameplayStatics.BreakHitResult` _outhit))
    (if (`KismetSystemLibrary.DoesImplementInterface` _hitactor "/Game/CoverMechanicThingy/BPI_GrowMoss.BPI_GrowMoss_C")
      (message `/Game/CoverMechanicThingy/BPI_GrowMoss.Grow Moss` _hitactor _returnvalue 200.0))))

(fn `UserConstructionScript`)