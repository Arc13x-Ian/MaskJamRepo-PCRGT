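; BPC_GravTrace is a component that moves its owning actor as a gravity-affected projectile using line traces.
; BeginPlay sets velocity from the owner's forward vector and speed, then destroys the owner after a delay.
; Each tick traces the next short segment with persistent debug drawing, snapping the owner to any hit.
; Otherwise, it advances to the segment's end and subtracts amplified gravity from velocity, producing an arc.
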(event `self.ReceiveBeginPlay`
  (set `self.Velocity` (* (`Actor.GetActorForwardVector` (`self.GetOwner`)) (`self.Speed`)))
  (set `self.Start Pos` (`Actor.K2_GetActorLocation` (`self.GetOwner`)))
  (`KismetSystemLibrary.Delay` 10.0)
  (`Actor.K2_DestroyActor` (`self.GetOwner`)))

(event `self.ReceiveTick`
  (params (DeltaSeconds :type "Float (single-precision)"))
  ; every tick get the start position FOR that tick, and then calculate an end position based on velocity and time
  (set `self.Delta Time` DeltaSeconds)
  (set `self.Start Pos` (`Actor.K2_GetActorLocation` (`self.GetOwner`)))
  (set `self.End Pos` (+ (`self.Start Pos`) (* (`self.Velocity`) (`self.Delta Time`))))
  (bind (_outhit _returnvalue) (`KismetSystemLibrary.LineTraceSingle` :`Start` (`self.Start Pos`) :`End` (`self.End Pos`) :`TraceChannel` "TraceTypeQuery1" :`DrawDebugType` "Persistent" :`DrawTime` 6.0))
  ; If we haven't hit anything yet, draw another trace, until we do.
  (if _returnvalue
    ; When we DO hit something, move the projectile location to the hit point
    (`Actor.K2_SetActorLocation` (`self.GetOwner`) (`.Location` (`GameplayStatics.BreakHitResult` _outhit)) false false)
    (else
      (`Actor.K2_SetActorLocation` (`self.GetOwner`) (`self.End Pos`) false false)
      (set `self.Velocity` (- (`self.Velocity`) (* (`KismetMathLibrary.MakeVector` 0.0 0.0 (* 980.0 10.0)) (`self.Delta Time`)))))))