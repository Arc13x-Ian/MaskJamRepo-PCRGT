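; Base seed actor that spawns a burst of BP_SeedProjectile actors to grow a plant.
; GrowPlant runs on BeginPlay and on overlap with a BP_WaterDroplet, which sets GotWatered so the new projectiles are flagged Watered.
; Each burst fires five projectiles from TargetPoint: one at the center and four offset and angled around it at 90-degree steps.
; A randomized-spread line trace remains in the graph but never runs.
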(event `self.ReceiveActorBeginOverlap`
  (params (OtherActor :type "Actor Object Reference"))
  (if (`KismetMathLibrary.ClassIsChildOf` (`GameplayStatics.GetObjectClass` OtherActor) "/Game/IanAssets/BP_WaterDroplet.BP_WaterDroplet_C")
    (set `self.GotWatered` true)
    (`self.GrowPlant`)))

(event `self.ReceiveBeginPlay`
  (`self.GrowPlant`))

(event `GrowPlant`
  (bind _returnvalue (`SceneComponent.K2_GetComponentLocation` (`self.TargetPoint`)))
  (for _index (range 5)
    (switch `int` _index
      (:`0`
        (set `self.Seed Spawner` (`KismetMathLibrary.MakeTransform` _returnvalue (struct :`Pitch` -90.0))))
      (:`1`
        (set `self.Seed Spawner` (`KismetMathLibrary.MakeTransform` (+ _returnvalue (5.0 0.0 5.0)) (struct :`Pitch` 80.0))))
      (:`2`
        (set `self.Seed Spawner` (`KismetMathLibrary.MakeTransform` (+ _returnvalue (0.0 5.0 5.0)) (struct :`Pitch` 80.0 :`Yaw` 90.0))))
      (:`3`
        (set `self.Seed Spawner` (`KismetMathLibrary.MakeTransform` (+ _returnvalue (-5.0 0.0 5.0)) (struct :`Pitch` 80.0 :`Yaw` 180.0))))
      (:`4`
        (set `self.Seed Spawner` (`KismetMathLibrary.MakeTransform` (+ _returnvalue (0.0 -5.0 5.0)) (struct :`Pitch` 80.0 :`Yaw` 270.0)))))
    (bind _returnvalue_2 (`|SpawnActorFromClass` "/Game/IanAssets/BP_SeedProjectile.BP_SeedProjectile_C" (`self.Seed Spawner`) "Undefined" "MultiplyWithRoot" null null))
    (if (`self.GotWatered`)
      (set `/Game/IanAssets/BP_SeedProjectile.watered` true _returnvalue_2))))

(fn `UserConstructionScript`)